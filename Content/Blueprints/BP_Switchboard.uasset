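; Switchboard actor with a panel that flips between a switches side and a buttons side, plus pressable Hold and Sorry buttons.
; Chained MoveComponentTo calls slide the panel along X, roll it half a turn and slide it back.
; BeginPlay turns the panel to the switches, and a separate event reverses the flip.
; Each button event pushes its component in and back out over configurable down and up times.
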(event Custom|RotateCToButtons
  (bind _sm_cpanel (Variables|Components|GetSM_CPanel))
  (Components|MoveComponentTo _sm_cpanel "10.000000,0.000000,0.000000" "0.000000,180.000000,0.000000" false true 0.2 false)
  (Components|MoveComponentTo _sm_cpanel "10.000000,0.000000,0.000000" "0, 0, 0" false false 0.3 false)
  (Components|MoveComponentTo _sm_cpanel "-15.000000,0.000000,0.000000" "0, 0, 0" true false 0.2 false))

(event Custom|PushButtonHold
  (bind _holdbuttonintern (Variables|Components|GetHoldButtonIntern))
  (Components|MoveComponentTo _holdbuttonintern "5.000000,0.000000,0.000000" "0, 0, 0" false false (Variables|Default|GetButtonDownTime) false)
  (Components|MoveComponentTo _holdbuttonintern "0, 0, 0" "0, 0, 0" false false (Variables|Default|GetButtonUpTime) false))

(event Custom|PushButtonSorry
  (bind _sorrybuttonintern (Variables|Components|GetSorryButtonIntern))
  (Components|MoveComponentTo _sorrybuttonintern "5.000000,0.000000,0.000000" "0, 0, 0" false false (Variables|Default|GetButtonDownTime) false)
  (Components|MoveComponentTo _sorrybuttonintern "0, 0, 0" "0, 0, 0" false false (Variables|Default|GetButtonUpTime) false))

(event Custom|RotateCToSwtitches
  (bind _sm_cpanel (Variables|Components|GetSM_CPanel))
  (Components|MoveComponentTo _sm_cpanel "10.000000,0.000000,0.000000" "0, 0, 0" false true 0.2 false)
  (Components|MoveComponentTo _sm_cpanel "10.000000,0.000000,0.000000" "0.000000,180.000000,0.000000" false false 0.3 false)
  (Components|MoveComponentTo _sm_cpanel "-15.000000,0.000000,0.000000" "0.000000,180.000000,0.000000" true false 0.2 false))

(event EventBeginPlay
  (CallFunction|RotateCtoSwtitches))

(event EventTick
  (params (DeltaSeconds :type Float%20%28single-precision%29)))

(fn ConstructionScript)